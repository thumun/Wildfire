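; BP_Firetruck is a firetruck with two abilities on hard-wired number keys for fighting fires on tiles.
; Key 1 toggles the water gun's Niagara effect; while active, Tick sphere-traces forward from WaterStartPos and calls TryExtinguishFire on hit BP_Tile actors.
; Key 2 calls Ability2, which spawns a BP_Sprinkler at the Niagara component's location, gated by a cooldown that Tick counts down.
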(event `Key|One`
  (params (Key :type "Key Structure"))
  (bind _niagara (`self.Niagara`))
  ;[1 1 1] Water gun
  (:`Pressed`
    (if (`self.Ability1Active`)
      (set `self.Ability1Active` false)
      (`ActorComponent.Deactivate` _niagara)
      (else
        (set `self.Ability1Active` true)
        (`ActorComponent.Activate` _niagara false)))))

(event `Key|Two`
  (params (Key :type "Key Structure"))
  ;[1 1 1] Place sprinkler
  (:`Pressed`
    (`self.Ability2`)))

(event `self.ReceiveTick`
  (params (DeltaSeconds :type "Float (single-precision)"))
  (bind _returnvalue (`SceneComponent.K2_GetComponentLocation` (`self.WaterStartPos`)))
  (set `self.Ability2Cooldown` (- (`self.Ability2Cooldown`) DeltaSeconds))
  (if (`self.Ability1Active`)
    ;[1 1 1] Fire extinguish logic
    (bind _outhits (`KismetSystemLibrary.SphereTraceMulti` _returnvalue (+ _returnvalue (* (`SceneComponent.GetForwardVector` (`self.WaterStartPos`)) 1000.0)) 200.0 "TraceTypeQuery1"))
    (for _array_element _outhits
      (bind _asbp_tile (cast `/Game/BP/BP_Tile` (`.HitActor` (`GameplayStatics.BreakHitResult` _array_element))))
      (`/Game/BP/BP_Tile.TryExtinguishFire` _asbp_tile))))

(fn `Ability2`
  (if (<= (`self.Ability2Cooldown`) 0.0)
    (`|SpawnActorFromClass` "/Game/BP/BP_Sprinkler.BP_Sprinkler_C" (`KismetMathLibrary.MakeTransform` (`SceneComponent.K2_GetComponentLocation` (`self.Niagara`))) "Undefined" "MultiplyWithRoot" null null)
    (set `self.Ability2Cooldown` 10.0)))

(fn `UserConstructionScript`
  (set `self.Ability1Active` false)
  (set `self.Ability2Cooldown` 0.0))