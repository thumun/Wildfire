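; Player-controlled Spark character with four abilities that act on tiles and draw on a regenerating fuel pool.
; Ability 1 toggles a material and drains fuel while igniting overlapped tiles; Ability 4 changes their state for a fuel cost.
; Ability 2 spawns a fan on cooldown; Ability 3 spends fuel to temporarily enlarge the box and boost speed.
; Tick runs timers and regeneration; the regen timer never resets after reaching its target.
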(event `self.ReceiveTick`
  (params (DeltaSeconds :type "Float (single-precision)"))
  (`self.UpdateAbilityTimes` DeltaSeconds)
  (if (and (<= (`self.Ability3ActiveTimer`) 0.0) (`self.Ability3Active`))
    (`self.Ability3` false))
  ;[1 1 1] Fuel Regeneration Logic
  (if (< (`self.FuelPoints`) 100.0)
    (bind _output_get (set `self.FuelRegenTimer` (+ DeltaSeconds (`self.FuelRegenTimer`))))
    (if (>= _output_get (`self.FuelRegenTargetTime`))
      (set `self.FuelPoints` (+ (`self.FuelPoints`) 5.0))))
  ;[1 1 1] Ability 1 Update
  (if (`self.Ability1Active`)
    (set `self.FuelPoints` (- (`self.FuelPoints`) (`self.Ability1CostRate`)))
    (for _array_element (`self.GetOverlappingActors` "/Game/BP/BP_Tile.BP_Tile_C")
      (bind _asbp_tile (cast `/Game/BP/BP_Tile` _array_element))
      (`/Game/BP/BP_Tile.TrySetFire` _asbp_tile))))

(event `self.ReceiveBeginPlay`)

(event `InputAxis|MoveForward`
  (params (AxisValue :type "Float (single-precision)"))
  ;[1 1 1] Movement
  (`self.AddMovementInput` (`self.GetActorForwardVector`) (* AxisValue (`self.MoveSpeed`))))

(event `InputAxis|Turn`
  (params (AxisValue :type "Float (single-precision)"))
  ;[1 1 1] Movement
  (`self.AddControllerYawInput` AxisValue))

(event `InputAction|A_1`
  (params (Key :type "Key Structure"))
  (:`Pressed`
    (if (`self.Ability1Active`)
      ;[1 1 1] Ability 1 Off
      (set `self.Ability1Active` false)
      (`PrimitiveComponent.SetMaterial` (`self.Spark`) 0 "/Game/Models/matSparkNeutral.matSparkNeutral")
      (elif (>= (`self.FuelPoints`) 5.0)
        ;[1 1 1] Ability 1 On
        (set `self.Ability1Active` true)
        (`PrimitiveComponent.SetMaterial` (`self.Spark`) 0 "/Game/Models/matSpark.matSpark")))))

(event `InputAction|A_2`
  (params (Key :type "Key Structure"))
  (:`Pressed`
    (`self.Ability2`)))

(event `InputAction|A_3`
  (params (Key :type "Key Structure"))
  (:`Pressed`
    (if (and (<= (`self.Ability3Cooldown`) 0.0) (<= (`self.Ability3Cost`) (`self.FuelPoints`)))
      (`self.Ability3` true))))

(event `InputAction|A_4`
  (params (Key :type "Key Structure"))
  (:`Pressed`
    (for _array_element (`self.GetOverlappingActors` "/Game/BP/BP_Tile.BP_Tile_C")
      (bind _asbp_tile (cast `/Game/BP/BP_Tile` _array_element))
      (bind _success (`/Game/BP/BP_Tile.ChangeState` _asbp_tile 3))
      (if _success
        (set `self.FuelPoints` (- (`self.FuelPoints`) (`self.Ability4Cost`)))))))

(fn `Ability2`
  (bind _fanspawnpoint (`self.FanSpawnPoint`))
  (if (<= (`self.Ability2Cooldown`) 0.0)
    (`|SpawnActorFromClass` "/Game/BP/BP_Fan.BP_Fan_C" (`KismetMathLibrary.MakeTransform` (`SceneComponent.K2_GetComponentLocation` _fanspawnpoint) (`KismetMathLibrary.Conv_VectorToRotator` (`SceneComponent.GetForwardVector` _fanspawnpoint))) "Undefined" "MultiplyWithRoot" null null)
    (set `self.Ability2Cooldown` 10.0)))

(fn `Ability3`
  (params (TurnOn :type Boolean))
  (if TurnOn
    (set `self.Ability3Active` true)
    (`SceneComponent.SetRelativeScale3D` (`self.Box`) (3.0 3.0 3.0))
    (set `self.MoveSpeed` 2.0)
    (set `self.Ability3ActiveTimer` 5.0)
    (set `self.Ability3Cooldown` 20.0)
    (set `self.FuelPoints` (- (`self.FuelPoints`) (`self.Ability3Cost`)))
    (else
      (set `self.Ability3Active` false)
      (`SceneComponent.SetRelativeScale3D` (`self.Box`) (1.0 1.0 1.0))
      (set `self.MoveSpeed` 1.0))))

(fn `UpdateAbilityTimes`
  (params (DeltaTime :type "Float (double-precision)"))
  (set `self.Ability2Cooldown` (- (`self.Ability2Cooldown`) DeltaTime))
  (set `self.Ability3Cooldown` (- (`self.Ability3Cooldown`) DeltaTime))
  (set `self.Ability3ActiveTimer` (- (`self.Ability3ActiveTimer`) DeltaTime)))

(fn `UserConstructionScript`
  (`PrimitiveComponent.SetMaterial` (`self.Spark`) 0 "/Game/Models/matSparkNeutral.matSparkNeutral")
  (set `self.FuelPoints` 100.0)
  (set `self.FuelRegenTimer` 0.0)
  (set `self.Ability1Active` false)
  (set `self.Ability3Active` false))