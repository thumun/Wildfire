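; BP_Tile is a grid tile that switches between neutral, burning and wet states, showing a matching component for each.
; While burning, a Tick timer periodically passes the tile's grid index to every BP_Grid actor to spread fire.
; A wet tile refuses TrySetFire until its wet timer expires and returns it to neutral.
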(event `self.ReceiveTick`
  (params (DeltaSeconds :type "Float (single-precision)"))
  (if (== (`self.state`) 1)
    ;[1 1 1] Fire spread
    (bind _output_get (set `self.spreadTimer` (+ (`self.spreadTimer`) DeltaSeconds)))
    (if (>= _output_get (`self.spreadTargetTime`))
      (`self.SpreadFire`)
      (set `self.spreadTimer` 0.0))
    (elif (and (== (`self.state`) 2) (`self.isWet`))
      ;[1 1 1] Wet duration
      (bind _output_get_2 (set `self.wetTimer` (+ (`self.wetTimer`) DeltaSeconds)))
      (if (>= _output_get_2 (`self.wetTargetTime`))
        (set `self.isWet` false)
        (`self.ChangeState` 0)))))

(fn `ChangeState`
  (params (NewState :type Integer))
  (bind _state (`self.state`))
  (if (and (!= NewState _state) (< _state 3))
    (switch `int` _state
      (:`Default`
        _)
      (:`0`
        (`SceneComponent.SetHiddenInGame` (`self.0Neutral`) true true))
      (:`1`
        (`SceneComponent.SetHiddenInGame` (`self.1Burning`) true true))
      (:`2`
        (`SceneComponent.SetHiddenInGame` (`self.2Wet`) true true)))
    (switch `int` NewState
      (:`Default`
        _)
      (:`0`
        (`SceneComponent.SetHiddenInGame` (`self.0Neutral`) false false))
      (:`1`
        (`SceneComponent.SetHiddenInGame` (`self.1Burning`) false false)
        (set `self.spreadTimer` 0.0))
      (:`2`
        (`SceneComponent.SetHiddenInGame` (`self.2Wet`) false false)
        (set `self.isWet` true)))
    (set `self.state` NewState)))

(fn `CurrentState`
  (returns (State :type Integer))
  (return (`self.state`)))

(fn `SetIndex`
  (params (index :type Integer))
  (set `self.gridIndex` index))

(fn `SpreadFire`
  (bind _outactors (`GameplayStatics.GetAllActorsOfClass` "/Game/BP/BP_Grid.BP_Grid_C"))
  (for _array_element _outactors
    (`/Game/BP/BP_Grid.SpreadFire` _array_element (`self.gridIndex`))))

(fn `TrySetFire`
  (if (not (`self.isWet`))
    (`self.ChangeState` 1)))

(fn `UserConstructionScript`
  (`self.ChangeState` 0)
  (set `self.spreadTimer` 0.0)
  (set `self.spreadTargetTime` 5.0)
  (set `self.isWet` false)
  (set `self.wetTimer` 0.0)
  (set `self.wetTargetTime` 5.0))