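; Level grid actor for a fire-spreading game, holding the BP_Tile board and reporting the burning fraction as score.
; The construction script spawns tiles and invisible border walls, placing obstacles and resources from EnviArray, a grid-ordered list rotated as entries are consumed.
; Fire spreads to orthogonal neighbours, or by fan along a cardinal direction, advanced on a Tick timer.
; Dev-only numpad keys force every tile's state.
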(event `Key|NumPadOne`
  (params (Key :type "Key Structure"))
  ;[1 1 1] DEV ONLY
  (:`Pressed`
    (for _array_element (`self.tileGrid`)
      (bind _asbp_tile (cast `/Game/BP/BP_Tile` _array_element))
      (`/Game/BP/BP_Tile.ChangeState` _asbp_tile 0))))

(event `self.ReceiveBeginPlay`)

(event `Key|NumPadTwo`
  (params (Key :type "Key Structure"))
  ;[1 1 1] DEV ONLY
  (:`Pressed`
    (for _array_element (`self.tileGrid`)
      (bind _asbp_tile (cast `/Game/BP/BP_Tile` _array_element))
      (`/Game/BP/BP_Tile.ChangeState` _asbp_tile 1))))

(event `Key|NumPadThree`
  (params (Key :type "Key Structure"))
  ;[1 1 1] DEV ONLY
  (:`Pressed`
    (for _array_element (`self.tileGrid`)
      (bind _asbp_tile (cast `/Game/BP/BP_Tile` _array_element))
      (`/Game/BP/BP_Tile.ChangeState` _asbp_tile 2))))

(event `self.ReceiveTick`
  (params (DeltaSeconds :type "Float (single-precision)"))
  (bind (_fanspreaddirection_x _fanspreaddirection_y) (`KismetMathLibrary.BreakVector` (`self.fanSpreadDirection`)))
  (bind _gridwidth (`self.gridWidth`))
  (bind _output_get (set `self.fanSpreadTimer` (- (`self.fanSpreadTimer`) DeltaSeconds)))
  (if (< _output_get 0.0)
    (set `self.fanSpreadTimer` 2.0)
    (for (_array_element _array_index) (`self.fanSpreadTiles`)
      ;[1 1 1] Spread fire towards fan direction
      (bind _asbp_tile (cast `/Game/BP/BP_Tile` (`|GetArrayItem` (`self.tileGrid`) _array_element)))
      (if (== (`/Game/BP/BP_Tile.state` _asbp_tile) 1)
        (bind _returnvalue (+ _array_element (+ _fanspreaddirection_x (* _fanspreaddirection_y _gridwidth))))
        (if (< _returnvalue (* (`self.gridHeight`) _gridwidth))
          (bind _asbp_tile_2 (cast `/Game/BP/BP_Tile` (`|GetArrayItem` (`self.tileGrid`) _returnvalue)))
          (`/Game/BP/BP_Tile.TrySetFire` _asbp_tile_2)
          (`KismetArrayLibrary.Array_Set` (`self.fanSpreadTiles`) _array_index _returnvalue))
        (else
          (`/Game/BP/BP_Tile.TrySetFire` _asbp_tile))))))

(fn `ComputeNewScore`
  (returns (FireScorePercent :type "Float (double-precision)"))
  (set `self.fireCount` 0)
  (for _array_element (`self.tileGrid`)
    (bind _asbp_tile (cast `/Game/BP/BP_Tile` _array_element))
    ;[1 1 1] Count number of burning blocks
    (bind _state (`/Game/BP/BP_Tile.CurrentState` _asbp_tile))
    (if (== _state 1)
      (set `self.fireCount` (+ 1 (`self.fireCount`)))))
  ;[1 1 1] Return the number of burning blocks as a fraction
  (return (/ (`KismetMathLibrary.Conv_IntToDouble` (`self.fireCount`)) (* (`self.gridWidth`) (`self.gridHeight`)))))

(fn `GetFirstElementArray`
  (params (EnviArr :type "Array of Vector Structure"))
  (returns (heightIndx :type Integer) (widthIndx :type Integer) (type :type Integer))
  (bind (_output_x _output_y _output_z) (`KismetMathLibrary.BreakVector` (`|GetArrayItem` EnviArr)))
  (return (`KismetMathLibrary.FTrunc` _output_x) (`KismetMathLibrary.FTrunc` _output_y) (`KismetMathLibrary.FTrunc` _output_z)))

(fn `LevelCreation`
  (params (Select :type Integer) (BPTile :type "/Game/BP/BP_Tile Object Reference"))
  (bind _obstaclecollider (`/Game/BP/BP_Tile.ObstacleCollider` BPTile))
  (bind _resourcecollider (`/Game/BP/BP_Tile.ResourceCollider` BPTile))
  (bind _obstaclemesh (`/Game/BP/BP_Tile.ObstacleMesh` BPTile))
  (bind _resourcemesh (`/Game/BP/BP_Tile.ResourceMesh` BPTile))
  (switch `int` Select
    (:`1`
      ;[1 1 1] Obstacle Spawning: (1 = tree, 2 = rock, 3  = water)
      (`PrimitiveComponent.SetCollisionEnabled` _obstaclecollider "QueryAndPhysics")
      (`StaticMeshComponent.SetStaticMesh` _obstaclemesh "/Game/Models/voxeltreenew.voxeltreenew")
      (`PrimitiveComponent.SetMaterial` _obstaclemesh 0 "/Game/Models/Material_001.Material_001")
      (`SceneComponent.SetVisibility` _obstaclemesh true true)
      (set `/Game/BP/BP_Tile.state` 5 BPTile :!label _label))
    (:`2`
      (`PrimitiveComponent.SetCollisionEnabled` _obstaclecollider "QueryAndPhysics")
      (`StaticMeshComponent.SetStaticMesh` _obstaclemesh "/Game/Models/newrock.newrock")
      (`PrimitiveComponent.SetMaterial` _obstaclemesh 0 "/Game/Models/Material_002.Material_002")
      (`SceneComponent.SetVisibility` _obstaclemesh true true)
      (goto _label))
    (:`3`
      (`PrimitiveComponent.SetCollisionEnabled` _obstaclecollider "QueryAndPhysics")
      (`SceneComponent.SetVisibility` (`/Game/BP/BP_Tile.GrassSprite` BPTile) false false)
      (`PrimitiveComponent.SetMaterial` (`/Game/BP/BP_Tile.DirtBox` BPTile) 0 "/Game/StarterContent/Materials/M_Water_Ocean.M_Water_Ocean")
      (goto _label))
    (:`4`
      ;[1 1 1] Resource Spawning: (4 = gas, 5 = water)
      (`PrimitiveComponent.SetCollisionEnabled` _resourcecollider "QueryAndPhysics")
      (`StaticMeshComponent.SetStaticMesh` _resourcemesh "/Game/Models/gasresource.gasresource")
      (`PrimitiveComponent.SetMaterial` _resourcemesh 0 "/Game/Models/DefaultMaterial.DefaultMaterial")
      (`SceneComponent.SetVisibility` _resourcemesh true true))
    (:`5`
      (`PrimitiveComponent.SetCollisionEnabled` _resourcecollider "QueryAndPhysics")
      (`StaticMeshComponent.SetStaticMesh` _resourcemesh "/Game/Models/waterresource.waterresource")
      (`PrimitiveComponent.SetMaterial` _resourcemesh 0 "/Game/Models/Plastic.Plastic")
      (`SceneComponent.SetVisibility` _resourcemesh true true)))
  (bind _outputarr (`self.RemoveFirstElementArray` (`self.enviArray`)))
  (set `self.enviArray` _outputarr)
  (return))

(fn `RemoveFirstElementArray`
  (params (InputArr :type "Array of Vector Structure"))
  (returns (OutputArr :type "Array of Vector Structure"))
  (for (_array_element _array_index) InputArr
    (if (== _array_index 0)
      (set `self.0thItem` _array_element)
      (else
        (`KismetArrayLibrary.Array_Set` InputArr (- _array_index 1) _array_element))))
  (`KismetArrayLibrary.Array_Set` InputArr (- (`KismetArrayLibrary.Array_Length` InputArr) 1) (`self.0thItem`)) ; 0th item at the end
  (return InputArr))

(fn `SpreadFireFan`
  (params (Index :type Integer) (SpreadDirection :type "Vector Structure"))
  (bind _returnvalue (< SpreadDirection_Y 0.0))
  (bind _returnvalue_2 (> SpreadDirection_X SpreadDirection_Y))
  (`KismetArrayLibrary.Array_Add` (`self.fanSpreadTiles`) Index)
  (set `self.fanSpreadTimer` 2.0)
  (if (< SpreadDirection_X 0.0)
    (if _returnvalue
      (if _returnvalue_2
        (set `self.fanSpreadDirection` (0.0 -1.0 0.0))
        (else
          (set `self.fanSpreadDirection` (-1.0 0.0 0.0))))
      (else
        (set `self.fanSpreadDirection` (0.0 1.0 0.0) :!label _label)))
    (else
      (if _returnvalue
        _
        (elif _returnvalue_2
          _
          (else
            (goto _label))))
      (set `self.fanSpreadDirection` (1.0 0.0 0.0)))))

(fn `SpreadFireOverTime`
  (params (index :type Integer))
  (if (< index (* (`self.gridWidth`) (- (`self.gridHeight`) 1)))
    ;[1 1 1] Spread fire above
    (bind _asbp_tile (cast `/Game/BP/BP_Tile` (`|GetArrayItem` (`self.tileGrid`) (+ index (`self.gridWidth`)))))
    (`/Game/BP/BP_Tile.TrySetFire` _asbp_tile))
  (if (>= index (`self.gridWidth`))
    ;[1 1 1] Spread fire below
    (bind _asbp_tile_2 (cast `/Game/BP/BP_Tile` (`|GetArrayItem` (`self.tileGrid`) (- index (`self.gridWidth`)))))
    (`/Game/BP/BP_Tile.TrySetFire` _asbp_tile_2))
  (if (> (mod index (`self.gridWidth`)) 0)
    ;[1 1 1] Spread fire left
    (bind _asbp_tile_3 (cast `/Game/BP/BP_Tile` (`|GetArrayItem` (`self.tileGrid`) (- index 1))))
    (`/Game/BP/BP_Tile.TrySetFire` _asbp_tile_3))
  (if true
    ;[1 1 1] Spread fire right
    (bind _asbp_tile_4 (cast `/Game/BP/BP_Tile` (`|GetArrayItem` (`self.tileGrid`) (+ index 1))))
    (`/Game/BP/BP_Tile.TrySetFire` _asbp_tile_4)))

(fn `UserConstructionScript`
  (bind _scale (`self.scale`))
  (bind _scale_2 (`self.scale`))
  (bind _scale_3 (`self.scale`))
  (bind _radius (`self.radius`))
  (bind _scale_4 (`self.scale`))
  (bind _scale_5 (`self.scale`))
  (bind _returnvalue (* 0.5 _radius 2.0))
  (bind _returnvalue_2 (* -1.0 _radius 2.0))
  (`StaticMeshComponent.SetStaticMesh` (`self.InstancedStaticMesh`) (`self.tileMesh`))
  (set `self.radius` (* (.x (`.Max` (break `Box` (`StaticMesh.GetBoundingBox` (`self.tileMesh`))))) (`self.scale`)))
  (for _index (range 1 (+ (`self.gridHeight`) 1))
    (bind _returnvalue_3 (- _index 1))
    (bind _returnvalue_4 (* _returnvalue_3 (`self.radius`) 2.0))
    ;[1 1 1] Invisible Walls Vertical
    (bind _returnvalue_5 (`AddComponent|NODE_AddChildActorComponent-1` :`RelativeTransform` (`KismetMathLibrary.MakeTransform` (`KismetMathLibrary.MakeVector` _returnvalue_2 _returnvalue_4 _returnvalue) (struct) (`KismetMathLibrary.MakeVector` _scale_4 _scale_4 1.0))))
    (`ChildActorComponent.SetChildActorClass` _returnvalue_5 "/Game/BP/BP_InvWall.BP_InvWall_C")
    (bind _returnvalue_6 (`AddComponent|NODE_AddChildActorComponent-3` :`RelativeTransform` (`KismetMathLibrary.MakeTransform` (`KismetMathLibrary.MakeVector` (* (`self.gridWidth`) 2.0 _radius) _returnvalue_4 _returnvalue) (struct) (`KismetMathLibrary.MakeVector` _scale_3 _scale_3 1.0))))
    (`ChildActorComponent.SetChildActorClass` _returnvalue_6 "/Game/BP/BP_InvWall.BP_InvWall_C")
    (for _index_2 (range 1 (+ (`self.gridWidth`) 1))
      (bind _returnvalue_7 (- _index_2 1))
      (bind _returnvalue_8 (* _returnvalue_7 (`self.radius`) 2.0))
      ;[1 1 1] Invisible Walls Horizontal
      (bind _returnvalue_9 (`AddComponent|NODE_AddChildActorComponent-2` :`RelativeTransform` (`KismetMathLibrary.MakeTransform` (`KismetMathLibrary.MakeVector` _returnvalue_8 _returnvalue_2 _returnvalue) (struct) (`KismetMathLibrary.MakeVector` _scale_5 _scale_5 1.0))))
      (`ChildActorComponent.SetChildActorClass` _returnvalue_9 "/Game/BP/BP_InvWall.BP_InvWall_C")
      (bind _returnvalue_10 (`AddComponent|NODE_AddChildActorComponent-4` :`RelativeTransform` (`KismetMathLibrary.MakeTransform` (`KismetMathLibrary.MakeVector` _returnvalue_8 (* (`self.gridHeight`) 2.0 _radius) _returnvalue) (struct) (`KismetMathLibrary.MakeVector` _scale _scale 1.0))))
      (`ChildActorComponent.SetChildActorClass` _returnvalue_10 "/Game/BP/BP_InvWall.BP_InvWall_C")
      ;[1 1 1] Child Actors
      (bind _returnvalue_11 (`AddComponent|NODE_AddChildActorComponent-0` :`RelativeTransform` (`KismetMathLibrary.MakeTransform` (`KismetMathLibrary.MakeVector` _returnvalue_8 _returnvalue_4) (struct) (`KismetMathLibrary.MakeVector` _scale_2 _scale_2 1.0))))
      (`ChildActorComponent.SetChildActorClass` _returnvalue_11 "/Game/BP/BP_Tile.BP_Tile_C")
      (bind _childactor (`ChildActorComponent.ChildActor` _returnvalue_11))
      (bind _returnvalue_12 (`KismetArrayLibrary.Array_Add` (`self.tileGrid`) _childactor))
      (bind _asbp_tile (cast `/Game/BP/BP_Tile` _childactor))
      (`/Game/BP/BP_Tile.SetIndex` _asbp_tile _returnvalue_12)
      (bind (_heightindx _widthindx _type) (`self.GetFirstElementArray` (`self.enviArray`)))
      (if (and (== _heightindx _returnvalue_3) (== _widthindx _returnvalue_7))
        (`self.LevelCreation` _type _asbp_tile)))))