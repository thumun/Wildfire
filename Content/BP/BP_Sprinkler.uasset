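; BP_Sprinkler is a temporary rotating sprinkler actor that puts out fires on nearby tiles and destroys itself when its lifetime runs out.
; A timeline started at BeginPlay drives the root's yaw, sweeping four arrow components that serve as spray directions.
; Every tick, it counts down the lifetime, sphere-traces forward from each arrow on the Visibility channel and calls TryExtinguishFire on any BP_Tile hit.
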(event `self.ReceiveBeginPlay`
  (bind (_direction _zrot) (`Timeline|Rotation`)
    (:`Update`
      (`SceneComponent.K2_SetRelativeRotation` (`self.DefaultSceneRoot`) (`KismetMathLibrary.MakeRotator` 0.0 0.0 _zrot) false false))))

(event `self.ReceiveTick`
  (params (DeltaSeconds :type "Float (single-precision)"))
  (bind _output_get (set `self.Deathtimer` (- (`self.Deathtimer`) DeltaSeconds)))
  (if (<= _output_get 0.0)
    (`self.K2_DestroyActor`)
    (else
      ;[1 1 1] Fire extinguish logic
      (for _array_element (`self.SprinklePos`)
        (bind _returnvalue (`SceneComponent.K2_GetComponentLocation` _array_element))
        (bind _outhits (`KismetSystemLibrary.SphereTraceMulti` _returnvalue (+ _returnvalue (* (`SceneComponent.GetForwardVector` _array_element) 500.0)) 100.0 "TraceTypeQuery1"))
        (for _array_element_2 _outhits
          (bind _asbp_tile (cast `/Game/BP/BP_Tile` (`.HitActor` (`GameplayStatics.BreakHitResult` _array_element_2))))
          (`/Game/BP/BP_Tile.TryExtinguishFire` _asbp_tile))))))

(fn `UserConstructionScript`
  (bind _sprinklepos (`self.SprinklePos`))
  (set `self.Deathtimer` 10.0)
  (`KismetArrayLibrary.Array_Add` _sprinklepos (`self.Arrow1`))
  (`KismetArrayLibrary.Array_Add` _sprinklepos (`self.Arrow2`))
  (`KismetArrayLibrary.Array_Add` _sprinklepos (`self.Arrow3`))
  (`KismetArrayLibrary.Array_Add` _sprinklepos (`self.Arrow4`)))