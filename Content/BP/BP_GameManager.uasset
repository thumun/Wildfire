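; BP_GameManager runs a timed match between Firetruck and Spark and decides the winner by fire score.
; Its construction script adds a BP_Grid child actor and initializes the match timers and state.
; Tick counts down the match and periodically refreshes the fire percentage by calling ComputeNewScore on grid actors.
; When time expires, it updates the score once more and prints Spark as winner at half or above, otherwise Firetruck.
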(event `self.ReceiveTick`
  (params (DeltaSeconds :type "Float (single-precision)"))
  (if (`self.isGameNotOver`)
    (bind _output_get (set `self.updateScoreTimer` (- (`self.updateScoreTimer`) DeltaSeconds)))
    (if (<= _output_get 0.0)
      (set `self.updateScoreTimer` 5.0)
      (`self.UpdateScore`))
    (bind _output_get_2 (set `self.remainingTime` (- (`self.remainingTime`) DeltaSeconds)))
    (if (<= _output_get_2 0.0)
      ;[1 1 1] Update score one last time and game over
      (`self.UpdateScore`)
      (`self.GameOver`))))

(fn `GameOver`
  (set `self.isGameNotOver` false)
  (if (< (`self.fireScorePercent`) 0.5)
    (`KismetSystemLibrary.PrintString` "Firetruck wins")
    (else
      (`KismetSystemLibrary.PrintString` "Spark wins"))))

(fn `UpdateScore`
  (bind _outactors (`GameplayStatics.GetAllActorsOfClass` "/Game/BP/BP_Grid.BP_Grid_C"))
  (for _array_element _outactors
    (bind _firescorepercent (`/Game/BP/BP_Grid.ComputeNewScore` _array_element))
    (bind _output_get (set `self.fireScorePercent` _firescorepercent))
    (`KismetSystemLibrary.PrintString` (`KismetStringLibrary.Conv_DoubleToString` _output_get))))

(fn `UserConstructionScript`
  (bind _returnvalue (`AddComponent|NODE_AddChildActorComponent-0` :`RelativeTransform` (`KismetMathLibrary.MakeTransform` (`self.spawnPos`))))
  (`ChildActorComponent.SetChildActorClass` _returnvalue "/Game/BP/BP_Grid.BP_Grid_C")
  (set `self.remainingTime` 300.0)
  (set `self.updateScoreTimer` 0.0)
  (set `self.isGameNotOver` true))