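; Menu player controller that handles the lobby and load screen UI, saved player profile and session exit back to the Menu level.
; Initial setup loads or creates the profile save, then passes it through ServerUpdateLobby to BP_Menu_Gamemode to refresh lobby names.
; Lobby and load screen widgets are created once and cached, with UpdatePlayerNames repopulating the lobby list.
; The local controller uses UI-only input with a visible cursor.
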(event `CreateLoadScreen`
  (`self.UI_ShowLoadScreen`))

(event `self.ReceiveBeginPlay`
  (if (`self.IsLocalController`)
    (set `self.bShowMouseCursor` true)
    (`WidgetBlueprintLibrary.SetInputMode_UIOnlyEx` self null)))

(event `EndClientSession`
  (`DestroySessionCallbackProxy.DestroySession` self
    (:`then`
      (`GameplayStatics.OpenLevelBySoftObjectPtr` "/Game/Levels/Menu/Menu.Menu"))))

(event `CreateLobbymenu`
  (`self.UI_ShowLobby`))

(event `UpdatePlayerNames`
  (params (PlayerProfs :type "Array of /Game/SavedData/S_PlayerProfile Structure"))
  (bind _lobbymenu (`self.LobbyMenu`))
  (`/Engine/EditorBlueprintResources/StandardMacros.IsValid` _lobbymenu
    (:`Is Valid`
      (`/Game/Widgets/W_LobbyMenu.ClearPlayerNames` _lobbymenu)
      (`/Game/Widgets/W_LobbyMenu.UpdatePlayerNames` _lobbymenu PlayerProfs))))

(event `Initial_Setup`
  (`self.LoadSavedProfile`)
  (`self.ServerUpdateLobby` (`self.Player Profile Info`)))

(event `ServerUpdateLobby`
  (params (`Player Profile` :type "/Game/SavedData/S_PlayerProfile Structure"))
  (set `self.Player Profile Info` `Player Profile`)
  (bind _asbp_menu_gamemode (cast `/Game/Framework/BP_Menu_Gamemode` (`GameplayStatics.GetGameMode`)))
  (`/Game/Framework/BP_Menu_Gamemode.UpdateLobby` _asbp_menu_gamemode true false))

(fn `LoadSavedProfile`
  (bind _returnvalue (`GameplayStatics.DoesSaveGameExist` (`self.Loc SlotName`)))
  (if (not _returnvalue)
    (bind _returnvalue_2 (`GameplayStatics.CreateSaveGameObject` "/Game/SavedData/SG_PlayerProfile.SG_PlayerProfile_C"))
    (`GameplayStatics.SaveGameToSlot` _returnvalue_2 (`self.Loc SlotName`)))
  (bind _returnvalue_3 (`GameplayStatics.LoadGameFromSlot` (`self.Loc SlotName`)))
  (bind _assg_player_profile (cast `/Game/SavedData/SG_PlayerProfile` _returnvalue_3))
  (set `self.Player Profile Info` (`/Game/SavedData/SG_PlayerProfile.PlayerProfile` _assg_player_profile))
  (return))

(fn `UI_ShowLoadScreen`
  (`WidgetLayoutLibrary.RemoveAllWidgets`)
  (`/Engine/EditorBlueprintResources/StandardMacros.IsValid` (`self.LoadScreen`)
    (:`Is Valid`
      _)
    (:`Is Not Valid`
      (bind _returnvalue (`|CreateWidget` "/Game/Widgets/W_LoadScreen.W_LoadScreen_C" self))
      (set `self.LoadScreen` _returnvalue)))
  (`UserWidget.AddToViewport` (`self.LoadScreen`) 0)
  (return))

(fn `UI_ShowLobby`
  (`/Engine/EditorBlueprintResources/StandardMacros.IsValid` (`self.LobbyMenu`)
    (:`Is Valid`
      _)
    (:`Is Not Valid`
      (bind _returnvalue (`|CreateWidget` "/Game/Widgets/W_LobbyMenu.W_LobbyMenu_C" self))
      (set `self.LobbyMenu` _returnvalue)))
  (`UserWidget.AddToViewport` (`self.LobbyMenu`) 0)
  (return))

(fn `UserConstructionScript`)