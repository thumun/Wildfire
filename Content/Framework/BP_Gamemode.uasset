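; Game mode for a wildfire versus firefighter game that spawns all players once the count expected by the game instance has joined.
; After a short delay it restarts each controller at the PlayerStart matching its join index and calls WaterGauge on the first one.
; The pawn spawn override alternates between WildFire and Firefighter test-child classes, starting from a random boolean set at BeginPlay.
; Tag-randomizing and profile-loading logic is left unconnected.
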(event `self.HandleStartingNewPlayer`
  (params (NewPlayer :type "PlayerController Object Reference"))
  (bind _asbp_player_controller (cast `/Game/Framework/BP_PlayerController` NewPlayer))
  (`KismetArrayLibrary.Array_Add` (`self.AllControllers`) _asbp_player_controller)
  (bind _asbp_game_instance (cast `/Game/Framework/BP_GameInstance` (`GameplayStatics.GetGameInstance`)))
  (set `self.Num Expected Players` (`/Game/Framework/BP_GameInstance.Num Players` _asbp_game_instance))
  (if (== (`self.Num Expected Players`) (`KismetArrayLibrary.Array_Length` (`self.AllControllers`)))
    (`KismetSystemLibrary.Delay` 0.5)
    (for (_array_element _array_index) (`self.AllControllers`)
      (if (not (`self.RandPicked`))
        (`/Game/Framework/BP_PlayerController.WaterGauge` _array_element)
        (set `self.RandPicked` true))
      (`self.RestartPlayerAtPlayerStart` _array_element (`self.K2_FindPlayerStart` _array_element (`KismetStringLibrary.Conv_IntToString` _array_index))))))

(event `self.ReceiveBeginPlay`
  (set `self.initialSpawn` (`KismetMathLibrary.RandomBool`)))

(fn `RandomNum`
  (returns (controller0 :type Integer) (controller1 :type Integer))
  (return (`self.TagNum`) (`self.TagNum_1`)))

(fn `SpawnDefaultPawnFor`
  (params (NewPlayer :type "Controller Object Reference") (StartSpot :type "Actor Object Reference"))
  (returns (ReturnValue :type "Pawn Object Reference"))
  (bind _returnvalue (`self.GetTransform` StartSpot))
  (bind _asbp_player_controller (cast `/Game/Framework/BP_PlayerController` NewPlayer))
  (bind _output_get (set `self.initialSpawn` (not (`self.initialSpawn`))))
  (if _output_get
    (bind _returnvalue_2 (`|SpawnActorFromClass` "/Game/BP/WildFireTESTCHILD.WildFireTESTCHILD_C" _returnvalue "Undefined" "MultiplyWithRoot" null null))
    (return _returnvalue_2)
    (else
      (bind _returnvalue_3 (`|SpawnActorFromClass` "/Game/BP/FirefighterTESTCHILD.FirefighterTESTCHILD_C" _returnvalue "Undefined" "MultiplyWithRoot" null null))
      (return _returnvalue_3))))

(fn `UserConstructionScript`)