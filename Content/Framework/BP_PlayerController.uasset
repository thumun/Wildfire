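; Player controller that gives the local player a role-specific HUD, either wildfire or firefighter.
; While the IsNotUI flag is set, Tick waits for a valid pawn, clears all widgets, picks the HUD by casting to WildFireTESTCHILD, sets game-only input, hides the cursor and clears the flag.
; Helper functions create each HUD widget if missing and add it to the player screen.
; FireGauge and WaterGauge events are empty stubs.
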(event `self.ReceiveBeginPlay`)

(event `self.ReceiveTick`
  (params (DeltaSeconds :type "Float (single-precision)"))
  (`/Engine/EditorBlueprintResources/StandardMacros.IsValid` (`self.K2_GetPawn`)
    (:`Is Valid`
      (if (`self.IsNotUI`)
        (if (`self.IsLocalPlayerController`)
          (`WidgetLayoutLibrary.RemoveAllWidgets`)
          (cast `/Game/BP/WildFireTESTCHILD` (`self.K2_GetPawn`)
            (:`then`
              (`self.UI_ShowInGameHUD`)
              (`WidgetBlueprintLibrary.SetInputMode_GameOnly` self)
              (set `self.bShowMouseCursor` false))
            (:`CastFailed`
              (`self.UI_ShowInGameHUDFirefighter`)
              (`WidgetBlueprintLibrary.SetInputMode_GameOnly` self)
              (set `self.bShowMouseCursor` false)))
          (set `self.IsNotUI` false))))))

(event `FireGauge`)

(event `WaterGauge`)

(fn `UI_ShowInGameHUD`
  (`/Engine/EditorBlueprintResources/StandardMacros.IsValid` (`self.WB_ingameHUD`)
    (:`Is Valid`
      _)
    (:`Is Not Valid`
      (bind _returnvalue (`|CreateWidget` "/Game/Widgets/W_InGameHUD.W_InGameHUD_C" self))
      (set `self.WB_ingameHUD` _returnvalue)))
  (`UserWidget.AddToPlayerScreen` (`self.WB_ingameHUD`) 0)
  (return))

(fn `UI_ShowInGameHUDFirefighter`
  (`/Engine/EditorBlueprintResources/StandardMacros.IsValid` (`self.WB_firefighterHUD`)
    (:`Is Valid`
      _)
    (:`Is Not Valid`
      (bind _returnvalue (`|CreateWidget` "/Game/Widgets/W_FirefighterHUD.W_FirefighterHUD_C" self))
      (set `self.WB_firefighterHUD` _returnvalue)))
  (`UserWidget.AddToPlayerScreen` (`self.WB_firefighterHUD`) 0)
  (return))

(fn `UserConstructionScript`)