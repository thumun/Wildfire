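; Game mode for the menu that manages players joining the Lobby level.
; When a new player starts in that level, it records their BP_Menucontroller, then has it create the lobby menu and run initial setup.
; When UpdateLobby is called with its PlayerNames flag set, it rebuilds the profile list from all recorded controllers and pushes it back to each one to update player names.
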(event `self.HandleStartingNewPlayer`
  (params (NewPlayer :type "PlayerController Object Reference"))
  (bind _returnvalue (`GameplayStatics.GetCurrentLevelName` true))
  (switch `string` _returnvalue
    (:`Lobby`
      (bind _asbp_menucontroller (cast `/Game/Framework/BP_Menucontroller` NewPlayer))
      (`KismetArrayLibrary.Array_Add` (`self.AllConnectedPlayers`) _asbp_menucontroller)
      (`/Game/Framework/BP_Menucontroller.CreateLobbymenu` _asbp_menucontroller)
      (`/Game/Framework/BP_Menucontroller.Initial_Setup` _asbp_menucontroller))))

(event `UpdateLobby`
  (params (PlayerNames :type Boolean))
  (if PlayerNames
    (`KismetArrayLibrary.Array_Clear` (`self.AllPlayerProfiles`))
    (for _array_element (`self.AllConnectedPlayers`)
      (`KismetArrayLibrary.Array_Add` (`self.AllPlayerProfiles`) (`/Game/Framework/BP_Menucontroller.Player Profile Info` _array_element)))
    (for _array_element_2 (`self.AllConnectedPlayers`)
      (if PlayerNames
        (`/Game/Framework/BP_Menucontroller.UpdatePlayerNames` _array_element_2 (`self.AllPlayerProfiles`))))))

(fn `UserConstructionScript`)